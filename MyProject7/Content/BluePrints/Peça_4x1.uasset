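; Blueprint for a 4x1 falling-block piece, apparently Tetris-style, that moves and rotates on a grid.
; Custom events shift the Peças component left, right or down in fixed steps, or rotate it a quarter turn either way.
; BeginPlay and Tick share a delayed loop that steps the piece downward while its movement base actor overlaps the owner of Peças.
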(event `Mover para Esquerda`
  (`SceneComponent.K2_AddLocalTransform` (`self.Peças`) (`KismetMathLibrary.MakeTransform` (-100.0 0.0 0.0)) false false))

(event `Mover Para Baixo`
  (`SceneComponent.K2_AddLocalTransform` (`self.Peças`) (`KismetMathLibrary.MakeTransform` (0.0 0.0 -100.0) (struct)) false false))

(event `Mover Anti Horario`
  (`SceneComponent.K2_AddLocalTransform` (`self.Peças`) (`KismetMathLibrary.MakeTransform` (0.0 0.0 0.0) (struct :`Pitch` -90.0)) false false))

(event `Key|K`
  (params (Key :type "Key Structure" :default "AnyKey")))

(event `InputAction|Esquerda`
  (params (Key :type "Key Structure" :default "AnyKey")))

(event `InputAction|Cima`
  (params (Key :type "Key Structure" :default "AnyKey")))

(event `Mover para Direita`
  (`SceneComponent.K2_AddLocalTransform` (`self.Peças`) (`KismetMathLibrary.MakeTransform` (100.0 0.0 0.0)) false false))

(event `Mover Horario`
  (`SceneComponent.K2_AddLocalTransform` (`self.Peças`) (`KismetMathLibrary.MakeTransform` (0.0 0.0 0.0) (struct :`Pitch` 90.0)) false false))

(event `self.ReceiveBeginPlay`
  (while (`self.IsOverlappingActor` (`Pawn.GetMovementBaseActor` null) (`ActorComponent.GetOwner` (`self.Peças`))) :!label _label
    (`KismetSystemLibrary.Delay` 0.5)
    (`SceneComponent.K2_AddLocalTransform` (`self.Peças`) (`KismetMathLibrary.MakeTransform` (0.0 0.0 -100.0)) false false)))

(event `self.ReceiveTick`
  (params (DeltaSeconds :type "Float (single-precision)"))
  (goto _label))

(fn `UserConstructionScript`)